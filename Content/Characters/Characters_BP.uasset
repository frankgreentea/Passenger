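; Interactable character Blueprint with up to six text bubbles, one clickable with hover colors, and a timed dialog window.
; The construction script sets the mesh and destroys surplus bubble components per NumberOfBuble; BeginPlay fills their text and hides them.
; DialogStart steps through DialogText with per-line delays, while Tick yaws the dialog window toward the camera.
; Separate events toggle bubble visibility, turn bubbles to the camera, and switch a custom-depth highlight.
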(event `KeepDialog_inView`
  (bind _dialog_window (`self.Dialog_Window`))
  (bind (_relativerotation_roll _relativerotation_pitch) (`KismetMathLibrary.BreakRotator` (`SceneComponent.RelativeRotation` _dialog_window)))
  (bind (_returnvalue_roll _returnvalue_pitch _returnvalue_yaw) (`KismetMathLibrary.BreakRotator` (`KismetMathLibrary.MakeRotFromX` (- (`SceneComponent.K2_GetComponentLocation` _dialog_window) (`self.K2_GetActorLocation` (`GameplayStatics.GetPlayerCameraManager` 0))))))
  (if (!= _dialog_window null)
    (`SceneComponent.K2_SetWorldRotation` _dialog_window (`KismetMathLibrary.MakeRotator` _relativerotation_roll _relativerotation_pitch (- _returnvalue_yaw 180.0)) false false)))

(event `DialogStart`
  (bind _linestate (`self.LineState`))
  (bind _linestate_2 (`self.LineState`))
  (`KismetSystemLibrary.Delay` (`|GetArrayItem` (`self.DelayBetweenLine`) _linestate) :!label _label)
  (bind _asbase_dialog_widget (cast `/Game/Base_dialog_Widget` (`WidgetComponent.GetUserWidgetObject` (`self.Dialog_Window`))))
  (`TextBlock.SetText` (`/Game/Base_dialog_Widget.dialog_Text` _asbase_dialog_widget) (`|GetArrayItem` (`self.DialogText`) _linestate_2))
  (if (not (>= _linestate_2 (`self.NumberOfLine`)))
    (set `self.LineState` (+ _linestate 1))
    (goto _label)))

(event `Texte_FacePlayer`
  (bind _widget_1 (`self.Widget_1`))
  (bind _widget_2 (`self.Widget_2`))
  (bind _widget_3 (`self.Widget_3`))
  (bind _widget_4 (`self.Widget_4`))
  (bind _widget_5 (`self.Widget_5`))
  (bind _widget_6_clickable (`self.Widget_6_Clickable`))
  (bind (_relativerotation_roll _relativerotation_pitch) (`KismetMathLibrary.BreakRotator` (`SceneComponent.RelativeRotation` _widget_6_clickable)))
  (bind (_relativerotation_roll_2 _relativerotation_pitch_2) (`KismetMathLibrary.BreakRotator` (`SceneComponent.RelativeRotation` _widget_1)))
  (bind (_relativerotation_roll_3 _relativerotation_pitch_3) (`KismetMathLibrary.BreakRotator` (`SceneComponent.RelativeRotation` _widget_2)))
  (bind (_relativerotation_roll_4 _relativerotation_pitch_4) (`KismetMathLibrary.BreakRotator` (`SceneComponent.RelativeRotation` _widget_3)))
  (bind (_relativerotation_roll_5 _relativerotation_pitch_5) (`KismetMathLibrary.BreakRotator` (`SceneComponent.RelativeRotation` _widget_4)))
  (bind (_relativerotation_roll_6 _relativerotation_pitch_6) (`KismetMathLibrary.BreakRotator` (`SceneComponent.RelativeRotation` _widget_5)))
  (bind (_returnvalue_roll _returnvalue_pitch _returnvalue_yaw) (`KismetMathLibrary.BreakRotator` (`KismetMathLibrary.MakeRotFromX` (- (`SceneComponent.K2_GetComponentLocation` _widget_3) (`self.K2_GetActorLocation` (`GameplayStatics.GetPlayerCameraManager` 0))))))
  (bind (_returnvalue_roll_2 _returnvalue_pitch_2 _returnvalue_yaw_2) (`KismetMathLibrary.BreakRotator` (`KismetMathLibrary.MakeRotFromX` (- (`SceneComponent.K2_GetComponentLocation` _widget_4) (`self.K2_GetActorLocation` (`GameplayStatics.GetPlayerCameraManager` 0))))))
  (bind (_returnvalue_roll_3 _returnvalue_pitch_3 _returnvalue_yaw_3) (`KismetMathLibrary.BreakRotator` (`KismetMathLibrary.MakeRotFromX` (- (`SceneComponent.K2_GetComponentLocation` _widget_5) (`self.K2_GetActorLocation` (`GameplayStatics.GetPlayerCameraManager` 0))))))
  (bind (_returnvalue_roll_4 _returnvalue_pitch_4 _returnvalue_yaw_4) (`KismetMathLibrary.BreakRotator` (`KismetMathLibrary.MakeRotFromX` (- (`SceneComponent.K2_GetComponentLocation` _widget_6_clickable) (`self.K2_GetActorLocation` (`GameplayStatics.GetPlayerCameraManager` 0))))))
  (bind (_returnvalue_roll_5 _returnvalue_pitch_5 _returnvalue_yaw_5) (`KismetMathLibrary.BreakRotator` (`KismetMathLibrary.MakeRotFromX` (- (`SceneComponent.K2_GetComponentLocation` _widget_1) (`self.K2_GetActorLocation` (`GameplayStatics.GetPlayerCameraManager` 0))))))
  (bind (_returnvalue_roll_6 _returnvalue_pitch_6 _returnvalue_yaw_6) (`KismetMathLibrary.BreakRotator` (`KismetMathLibrary.MakeRotFromX` (- (`SceneComponent.K2_GetComponentLocation` _widget_2) (`self.K2_GetActorLocation` (`GameplayStatics.GetPlayerCameraManager` 0))))))
  (if (!= _widget_1 null)
    (`SceneComponent.K2_SetWorldRotation` _widget_1 (`KismetMathLibrary.MakeRotator` _relativerotation_roll_2 _relativerotation_pitch_2 (- _returnvalue_yaw_5 180.0)) false false))
  (if (!= _widget_2 null)
    (`SceneComponent.K2_SetRelativeRotation` _widget_2 (`KismetMathLibrary.MakeRotator` _relativerotation_roll_3 _relativerotation_pitch_3 (- _returnvalue_yaw_6 180.0)) false false))
  (if (!= _widget_3 null)
    (`SceneComponent.K2_SetRelativeRotation` _widget_3 (`KismetMathLibrary.MakeRotator` _relativerotation_roll_4 _relativerotation_pitch_4 (- _returnvalue_yaw 180.0)) false false))
  (if (!= _widget_4 null)
    (`SceneComponent.K2_SetRelativeRotation` _widget_4 (`KismetMathLibrary.MakeRotator` _relativerotation_roll_5 _relativerotation_pitch_5 (- _returnvalue_yaw_2 180.0)) false false))
  (if (!= _widget_5 null)
    (`SceneComponent.K2_SetRelativeRotation` _widget_5 (`KismetMathLibrary.MakeRotator` _relativerotation_roll_6 _relativerotation_pitch_6 (- _returnvalue_yaw_3 180.0)) false false))
  (if (!= _widget_6_clickable null)
    (`SceneComponent.K2_SetRelativeRotation` _widget_6_clickable (`KismetMathLibrary.MakeRotator` _relativerotation_roll _relativerotation_pitch (- _returnvalue_yaw_4 180.0)) false false)))

(event `Clickable_Unhovered`
  (bind _asbase_widget (cast `/Game/Base_Widget` (`WidgetComponent.GetUserWidgetObject` (`self.Widget_6_Clickable`))))
  (`TextBlock.SetColorAndOpacity` (`/Game/Base_Widget.Text_block` _asbase_widget) (make `SlateColor` (`KismetMathLibrary.Conv_ColorToLinearColor` (`self.ClickableColor`)))))

(event `Clickable_Hover`
  (bind _asbase_widget (cast `/Game/Base_Widget` (`WidgetComponent.GetUserWidgetObject` (`self.Widget_6_Clickable`))))
  (`TextBlock.SetColorAndOpacity` (`/Game/Base_Widget.Text_block` _asbase_widget) (make `SlateColor` (`KismetMathLibrary.Conv_ColorToLinearColor` (`self.Clockable_HoverColor`)))))

(event `self.ReceiveBeginPlay`
  ;[1 1 1] Begin
  (`PrimitiveComponent.SetCustomDepthStencilValue` (`self.SkeletalMesh`) 1)
  (`self.TextAssignement`)
  (`self.Visibility_OFf`)
  (if (`self.Clickable_Choice`)
    (bind _asbase_widget (cast `/Game/Base_Widget` (`WidgetComponent.GetUserWidgetObject` (`self.Widget_6_Clickable`))))
    (`TextBlock.SetColorAndOpacity` (`/Game/Base_Widget.Text_block` _asbase_widget) (make `SlateColor` (`KismetMathLibrary.Conv_ColorToLinearColor` (`self.ClickableColor`))))
    (set `/Game/Base_Widget.TextColor_Normal` (`self.ClickableColor`) _asbase_widget)
    (set `/Game/Base_Widget.TextColor_Hovered` (`self.Clockable_HoverColor`) _asbase_widget)
    (bind _asbase_dialog_widget (cast `/Game/Base_dialog_Widget` (`WidgetComponent.GetUserWidgetObject` (`self.Dialog_Window`))))
    (`TextBlock.SetColorAndOpacity` (`/Game/Base_dialog_Widget.dialog_Text` _asbase_dialog_widget) (make `SlateColor` (`KismetMathLibrary.Conv_ColorToLinearColor` (`self.Dialog_Color`))))))

(event `Interactible_Feedback_On`
  ;[1 1 1] Feedack Outline
  (`PrimitiveComponent.SetRenderCustomDepth` (`self.SkeletalMesh`) true))

(event `Interactible_Feedback_off`
  ;[1 1 1] Feedack Outline
  (`PrimitiveComponent.SetRenderCustomDepth` (`self.SkeletalMesh`) false))

(event `self.ReceiveTick`
  (params (DeltaSeconds :type "Float (single-precision)"))
  (`self.KeepDialog_inView`))

(event `TextAssignement`
  (switch `int` (`self.number of buble`)
    (:`1`
      _)
    (:`2`
      (bind _asbase_widget (cast `/Game/Base_Widget` (`WidgetComponent.GetUserWidgetObject` (`self.Widget_1`)) :!label _label_2))
      (`TextBlock.SetText` (`/Game/Base_Widget.Text_block` _asbase_widget) (`self.Text1`)))
    (:`3`
      (bind _asbase_widget_2 (cast `/Game/Base_Widget` (`WidgetComponent.GetUserWidgetObject` (`self.Widget_5`)) :!label _label_3))
      (`TextBlock.SetText` (`/Game/Base_Widget.Text_block` _asbase_widget_2) (`self.TEXT5`))
      (goto _label_2))
    (:`4`
      (bind _asbase_widget_3 (cast `/Game/Base_Widget` (`WidgetComponent.GetUserWidgetObject` (`self.Widget_4`)) :!label _label_4))
      (`TextBlock.SetText` (`/Game/Base_Widget.Text_block` _asbase_widget_3) (`self.TEXT4`))
      (goto _label_3))
    (:`5`
      (bind _asbase_widget_4 (cast `/Game/Base_Widget` (`WidgetComponent.GetUserWidgetObject` (`self.Widget_3`)) :!label _label_5))
      (`TextBlock.SetText` (`/Game/Base_Widget.Text_block` _asbase_widget_4) (`self.TEXT3`))
      (goto _label_4))
    (:`6`
      (bind _asbase_widget_5 (cast `/Game/Base_Widget` (`WidgetComponent.GetUserWidgetObject` (`self.Widget_2`))))
      (`TextBlock.SetText` (`/Game/Base_Widget.Text_block` _asbase_widget_5) (`self.TEXT2`))
      (goto _label_5)))
  (bind _asbase_widget_6 (cast `/Game/Base_Widget` (`WidgetComponent.GetUserWidgetObject` (`self.Widget_6_Clickable`))))
  (`TextBlock.SetText` (`/Game/Base_Widget.Text_block` _asbase_widget_6) (`self.TEXT6_Clickable`)))

(event `Visible_On`
  (bind _widget_2 (`self.Widget_2`))
  (bind _widget_3 (`self.Widget_3`))
  (bind _widget_4 (`self.Widget_4`))
  (bind _widget_5 (`self.Widget_5`))
  (bind _widget_6_clickable (`self.Widget_6_Clickable`))
  (bind _widget_1 (`self.Widget_1`))
  ;[1 1 1] Choice_Buble
  (if (not (== _widget_2 null))
    (`SceneComponent.SetVisibility` _widget_2 true false))
  (if (not (== _widget_3 null))
    (`SceneComponent.SetVisibility` _widget_3 true false))
  (if (not (== _widget_4 null))
    (`SceneComponent.SetVisibility` _widget_4 true false))
  (if (not (== _widget_5 null))
    (`SceneComponent.SetVisibility` _widget_5 true false))
  (if (not (== _widget_6_clickable null))
    (`SceneComponent.SetVisibility` _widget_6_clickable true false))
  (if (not (== _widget_1 null))
    (`SceneComponent.SetVisibility` _widget_1 true false)))

(event `Visibility_OFf`
  (bind _widget_2 (`self.Widget_2`))
  (bind _widget_4 (`self.Widget_4`))
  (bind _widget_5 (`self.Widget_5`))
  (bind _widget_6_clickable (`self.Widget_6_Clickable`))
  (bind _widget_1 (`self.Widget_1`))
  (bind _widget_3 (`self.Widget_3`))
  ;[1 1 1] Choice_Buble
  (if (not (== _widget_2 null))
    (`SceneComponent.SetVisibility` _widget_2 false false))
  (if (not (== _widget_3 null))
    (`SceneComponent.SetVisibility` _widget_3 false false))
  (if (not (== _widget_4 null))
    (`SceneComponent.SetVisibility` _widget_4 false false))
  (if (not (== _widget_5 null))
    (`SceneComponent.SetVisibility` _widget_5 false false))
  (if (not (== _widget_6_clickable null))
    (`SceneComponent.SetVisibility` _widget_6_clickable false false))
  (if (not (== _widget_1 null))
    (`SceneComponent.SetVisibility` _widget_1 false false)))

(fn `UserConstructionScript`
  (`SkinnedMeshComponent.SetSkinnedAssetAndUpdate` (`self.SkeletalMesh`) (`self.Mesh`) true)
  (switch `int` (`self.number of buble`)
    (:`1`
      (`ActorComponent.K2_DestroyComponent` (`self.Widget_2`))
      (`ActorComponent.K2_DestroyComponent` (`self.Widget_3`) :!label _label)
      (`ActorComponent.K2_DestroyComponent` (`self.Widget_4`) :!label _label_2)
      (`ActorComponent.K2_DestroyComponent` (`self.Widget_5`) :!label _label_3))
    (:`2`
      (goto _label))
    (:`3`
      (goto _label_2))
    (:`4`
      (goto _label_3))
    (:`5`
      _))
  (`ActorComponent.K2_DestroyComponent` (`self.Widget_1`)))